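; Base hideout interface actor that reveals its name display when the player character is nearby.
; The construction script writes the Name variable into a text render component.
; Overlap on ConfirmArea with BP_PlayerMainCharacter triggers a timeline that scales the Scene component up from zero, reversing it when the overlap ends.
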(event `self.ReceiveBeginPlay`
  (`SceneComponent.SetWorldScale3D` (`self.Scene`) (0.0 0.0 0.0)))

(event `self.ConfirmArea.OnComponentBeginOverlap`
  (params (OverlappedComponent :type "PrimitiveComponent Object Reference") (OtherActor :type "Actor Object Reference") (OtherComp :type "PrimitiveComponent Object Reference") (OtherBodyIndex :type Integer) (bFromSweep :type Boolean) (SweepResult :type "HitResult Structure (by ref)"))
  (cast `/Game/Anim/BluePrint_ZAP/BP_PlayerMainCharacter` OtherActor)
  (`self.ShowName`))

(event `self.ConfirmArea.OnComponentEndOverlap`
  (params (OverlappedComponent :type "PrimitiveComponent Object Reference") (OtherActor :type "Actor Object Reference") (OtherComp :type "PrimitiveComponent Object Reference") (OtherBodyIndex :type Integer))
  (cast `/Game/Anim/BluePrint_ZAP/BP_PlayerMainCharacter` OtherActor)
  (`self.UnShowName`))

(event `ShowName`
  (bind (_direction _alpha) (`Timeline|ShwoNameTimeline` :!via `PlayFromStart` :!label _label)
    (:`Update`
      (`SceneComponent.SetWorldScale3D` (`self.Scene`) (`KismetMathLibrary.VLerp` (0.0 0.0 0.0) (1.0 2.75 2.75) _alpha)))))

(event `UnShowName`
  (goto _label :!via `ReverseFromEnd`))

(fn `UserConstructionScript`
  (`TextRenderComponent.K2_SetText` (`self.TextRender`) (`self.Name`)))