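; Base city tile that spawns a building at its location and scatters random pickups around it on BeginPlay.
; The construction script gathers four marker positions, each of which gets a health, M4 or Uzi GPI through the spawner component, with health twice as likely.
; Every Tick, line traces along four arrows, ignoring city generator actors, show each road mesh only when something blocks that direction.
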(event `self.ReceiveBeginPlay`
  (`|ExecutionSequence`
    (:`then_0`
      (bind _returnvalue (`|SpawnActorFromClass` (`self.BuildingBaseClass`) (`KismetMathLibrary.MakeTransform` (`self.K2_GetActorLocation`)) "Undefined" "SelectDefaultAtRuntime" null null))
      (set `self.BuildingRef` _returnvalue))
    (:`then_1`
      (for _array_element (`self.GPISpawnerPos`)
        (`self.RandomPickUpAGPIClass` _array_element)))))

(event `self.ReceiveTick`
  (params (DeltaSeconds :type "Float (single-precision)"))
  (`self.CheckIfNeedRoad`))

(fn `AdjustIfTheRoadShown`
  (params (TargetActor :type "ArrowComponent Object Reference") (RoadMesh :type "StaticMeshComponent Object Reference"))
  (bind _returnvalue (`SceneComponent.K2_GetComponentLocation` TargetActor))
  (bind _outactors (`GameplayStatics.GetAllActorsOfClass` "/Game/MonsterCage_HWH/BP/Generater/BP_Cityenerator.BP_Cityenerator_C"))
  (bind _outhit (`KismetSystemLibrary.LineTraceSingle` _returnvalue (+ _returnvalue (* (`KismetMathLibrary.GetForwardVector` (`SceneComponent.K2_GetComponentRotation` TargetActor)) 1000.0)) "TraceTypeQuery1" false _outactors))
  (if (`GameplayStatics.BreakHitResult` _outhit)
    (`SceneComponent.SetHiddenInGame` RoadMesh false false)
    (else
      (`SceneComponent.SetHiddenInGame` RoadMesh true false))))

(fn `CheckIfNeedRoad`
  (`self.AdjustIfTheRoadShown` (`self.Arrow`) (`self.Cube`))
  (`self.AdjustIfTheRoadShown` (`self.Arrow1`) (`self.Cube1`))
  (`self.AdjustIfTheRoadShown` (`self.Arrow2`) (`self.Cube2`))
  (`self.AdjustIfTheRoadShown` (`self.Arrow3`) (`self.Cube3`)))

(fn `RandomPickUpAGPIClass`
  (params (WorldLocation :type "Vector Structure"))
  (locals (SpawnLocation :type "Vector Structure"))
  (set `local.SpawnLocation` WorldLocation)
  (switch `int` (`KismetMathLibrary.RandomIntegerInRange` 1 4)
    (:`1`
      (`/Game/MonsterCage_HWH/BP/Component/BPC_GPISpawner.SpawnGPI` (`self.BPC_GPISpawner`) "/Game/source/GPI_spawner/GPI/GPI_items/GPI_HP.GPI_HP_C" (`local.SpawnLocation`)))
    (:`2`
      (`/Game/MonsterCage_HWH/BP/Component/BPC_GPISpawner.SpawnGPI` (`self.BPC_GPISpawner`) "/Game/source/GPI_spawner/GPI/GPI_items/GPI_m4.GPI_m4_C" (`local.SpawnLocation`)))
    (:`3`
      (`/Game/MonsterCage_HWH/BP/Component/BPC_GPISpawner.SpawnGPI` (`self.BPC_GPISpawner`) "/Game/source/GPI_spawner/GPI/GPI_items/GPI_uzi.GPI_uzi_C" (`local.SpawnLocation`)))
    (:`4`
      (`/Game/MonsterCage_HWH/BP/Component/BPC_GPISpawner.SpawnGPI` (`self.BPC_GPISpawner`) "/Game/source/GPI_spawner/GPI/GPI_items/GPI_HP.GPI_HP_C" (`local.SpawnLocation`)))))

(fn `UserConstructionScript`
  (`KismetArrayLibrary.Array_Add` (`self.GPISpawnerPos`) (`SceneComponent.K2_GetComponentLocation` (`self.GPIpos`)))
  (`KismetArrayLibrary.Array_Add` (`self.GPISpawnerPos`) (`SceneComponent.K2_GetComponentLocation` (`self.GPIpos1`)))
  (`KismetArrayLibrary.Array_Add` (`self.GPISpawnerPos`) (`SceneComponent.K2_GetComponentLocation` (`self.GPIpos2`)))
  (`KismetArrayLibrary.Array_Add` (`self.GPISpawnerPos`) (`SceneComponent.K2_GetComponentLocation` (`self.GPIpos3`))))