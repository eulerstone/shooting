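; BP_BuildingBase is a base building actor that generates a randomly sized and colored placeholder building.
; The construction script randomizes the mesh scale, with an extra multiplier on height, then offsets Z by 50 times that scale.
; It also creates a dynamic material instance from M_Base with a random BaseColor.
; The SelectThisBuilding event only switches the BuildingSignState enum to one fixed value.
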(event `SelectThisBuilding`
  (set `self.BuildingSignState` "NewEnumerator2"))

(fn `UserConstructionScript`
  (bind (_returnvalue_x _returnvalue_y _returnvalue_z) (`KismetMathLibrary.BreakVector` (`SceneComponent.K2_GetComponentScale` (`self.Building`))))
  (bind _returnvalue (`KismetMathLibrary.RandomFloatInRange` (`self.ScaleRangeMin_PH`) (`self.ScaleRangMax_PH`)))
  (`SceneComponent.SetWorldScale3D` (`self.Building`) (`KismetMathLibrary.MakeVector` _returnvalue _returnvalue (`KismetMathLibrary.RandomFloatInRange` (* (`self.ScaleRangeMin_PH`) (`self.ZMulti_Temp`)) (* (`self.ScaleRangMax_PH`) (`self.ZMulti_Temp`)))))
  (bind _returnvalue_2 (`PrimitiveComponent.CreateDynamicMaterialInstance` (`self.Building`) 0 "/Game/MonsterCage_HWH/MAt/M_Base.M_Base" "None"))
  (bind _output_get (set `self.MI` _returnvalue_2))
  (`MaterialInstanceDynamic.SetVectorParameterValue` _output_get "BaseColor" (make `LinearColor` (`KismetMathLibrary.RandomFloatInRange` 0.0 1.0) (`KismetMathLibrary.RandomFloatInRange` 0.0 1.0) (`KismetMathLibrary.RandomFloatInRange` 0.0 1.0)))
  (`SceneComponent.K2_SetRelativeLocation` (`self.Building`) (`KismetMathLibrary.MakeVector` 0.0 0.0 (* _returnvalue_z 50.0)) false false))